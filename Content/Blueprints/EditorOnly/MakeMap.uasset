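; MakeMap is an actor in the EditorOnly folder that builds an empty world from a chain of spawned floor pieces.
; SpawnEmptyWorld clears the previous floors through RemoveFloors, then loops over NumberOfFloors, calling AddFloor and storing each result in Floors.
; AddFloor spawns the Floor class at NextSpawnPoint, then takes that piece's attach transform as the next spawn point.
; RemoveFloors destroys all stored pieces and resets the spawn point to the world origin.
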(event `SpawnEmptyWorld`
  (`self.RemoveFloors`)
  (for _ (range (+ (`self.NumberOfFloors`) 1))
    (bind _madefloor (`self.AddFloor` "/Game/Blueprints/Floors/Floor.Floor_C"))
    (`KismetArrayLibrary.Array_Add` (`self.Floors`) _madefloor)))

(event `RemoveFloors`
  (bind _floors (`self.Floors`))
  (for _array_element _floors
    (`self.K2_DestroyActor` _array_element))
  (`KismetArrayLibrary.Array_Clear` _floors)
  (set `self.NextSpawnPoint` (`KismetMathLibrary.MakeTransform` (0.0 0.0 0.0))))

(fn `AddFloor`
  (params (Floor :type "/Game/Blueprints/Floors/Floor Class Reference"))
  (returns (MadeFloor :type "/Game/Blueprints/Floors/Floor Object Reference"))
  (bind _returnvalue (`|SpawnActorFromClass` Floor (`self.NextSpawnPoint`) "Undefined" "OverrideRootScale" null null))
  (bind _attachtransform (`/Game/Blueprints/Floors/Floor.GetAttachTransform` _returnvalue))
  (set `self.NextSpawnPoint` _attachtransform)
  (return _returnvalue))

(fn `UserConstructionScript`)