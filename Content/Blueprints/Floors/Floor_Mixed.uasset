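; Endless-style floor segment that fills itself with a random mix of points, meteors and black holes.
; Spawn places a random formation class at a random offset and yaw as a temporary layout template.
; SpawnFormation swaps its name-prefixed arrow components for tracked actors, then destroys the template.
; When RayCharacter leaves EndTrigger, it requests another floor from RayGameMode if Procedural, then destroys itself and its actors after a delay.
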(event `self.ReceiveBeginPlay`)

(event `Spawn`
  (bind _returnvalue (`|SpawnActorFromClass` (`|GetArrayItem` (`self.Formations`) (`KismetMathLibrary.RandomInteger` (`KismetArrayLibrary.Array_Length` (`self.Formations`)))) (`KismetMathLibrary.MakeTransform` (+ (`KismetMathLibrary.MakeVector` (`KismetMathLibrary.RandomFloatInRange` 0.0 450.0) (`KismetMathLibrary.RandomFloatInRange` -450.0 450.0)) (.location (`self.GetTransform`))) (`KismetMathLibrary.MakeRotator` (.roll (.rotation (`self.GetTransform`))) (.pitch (.rotation (`self.GetTransform`))) (`KismetMathLibrary.RandomFloatInRange` -130.0 130.0)) (.scale (`self.GetTransform`))) "Undefined" "OverrideRootScale" null null))
  (`self.SpawnFormation` _returnvalue))

(event `self.EndTrigger.OnComponentEndOverlap`
  (params (OverlappedComponent :type "PrimitiveComponent Object Reference") (OtherActor :type "Actor Object Reference") (OtherComp :type "PrimitiveComponent Object Reference") (OtherBodyIndex :type Integer))
  (bind _mythings (`self.MyThings`))
  (cast `/Game/Blueprints/RayCharacter` OtherActor)
  (`/Engine/EditorBlueprintResources/StandardMacros.DoOnce` false
    (:`Completed`
      (if (`self.Procedural`)
        (bind _asray_game_mode (cast `/Game/Blueprints/RayGameMode` (`GameplayStatics.GetGameMode`)))
        (`/Game/Blueprints/RayGameMode.AddRandomFloor` _asray_game_mode))
      (`KismetSystemLibrary.Delay` 4.0)
      (for (_array_element _array_index) _mythings
        (`/Engine/EditorBlueprintResources/StandardMacros.IsValid` _array_element
          (:`Is Valid`
            (`self.K2_DestroyActor` (`|GetArrayItem` _mythings _array_index)))))
      (`KismetArrayLibrary.Array_Clear` _mythings)
      (`self.K2_DestroyActor`))))

(fn `SpawnFormation`
  (params (Formation :type "/Game/Blueprints/Floors/MixedPrefabs/Formation Object Reference"))
  (locals (GivenFormation :type "/Game/Blueprints/Floors/MixedPrefabs/Formation Object Reference"))
  (bind _output_get (set `local.GivenFormation` Formation))
  (for _array_element (`self.K2_GetComponentsByClass` _output_get "/Script/Engine.ArrowComponent")
    (switch `string` (`KismetStringLibrary.Left` (`KismetSystemLibrary.GetObjectName` _array_element) 6)
      (:`SpawnP`
        (bind (_returnvalue_location _returnvalue_rotation _returnvalue_scale) (`KismetMathLibrary.BreakTransform` (`SceneComponent.K2_GetComponentToWorld` _array_element)))
        (bind _returnvalue (`KismetMathLibrary.MakeTransform` _returnvalue_location (struct) _returnvalue_scale))
        (bind _returnvalue_2 (`|SpawnActorFromClass` "/Game/Blueprints/Points/Point.Point_C" _returnvalue "Undefined" "OverrideRootScale" null null))
        (`KismetArrayLibrary.Array_Add` (`self.MyThings`) _returnvalue_2))
      (:`SpawnM`
        (bind _returnvalue_3 (`|SpawnActorFromClass` "/Game/Blueprints/Obstacles/Meteor.Meteor_C" _returnvalue "Undefined" "OverrideRootScale" null null))
        (`KismetArrayLibrary.Array_Add` (`self.MyThings`) _returnvalue_3))
      (:`SpawnB`
        (bind _returnvalue_4 (`|SpawnActorFromClass` "/Game/Blueprints/Obstacles/BlackHole.BlackHole_C" _returnvalue "Undefined" "OverrideRootScale" null null))
        (`KismetArrayLibrary.Array_Add` (`self.MyThings`) _returnvalue_4))))
  (`self.K2_DestroyActor` (`local.GivenFormation`)))

(fn `UserConstructionScript`
  (`parent.UserConstructionScript`))