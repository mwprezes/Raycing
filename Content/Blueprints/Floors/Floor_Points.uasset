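; Floor segment that fills itself with point pickups and extends the level as the player passes through.
; On BeginPlay it spawns a random PointFormation at a random offset, using its arrow components as markers for spawning points, then destroys the formation.
; When RayCharacter first leaves EndTrigger, a procedural floor asks RayGameMode for another random floor.
; After a short delay, any floor destroys its remaining points and itself.
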(event `self.ReceiveBeginPlay`
  ;[1 1 1] Procedural
  (bind _returnvalue (`|SpawnActorFromClass` (`|GetArrayItem` (`self.Formations`) (`KismetMathLibrary.RandomInteger` (`KismetArrayLibrary.Array_Length` (`self.Formations`)))) (`KismetMathLibrary.MakeTransform` (+ (`KismetMathLibrary.MakeVector` (`KismetMathLibrary.RandomFloatInRange` 0.0 450.0) (`KismetMathLibrary.RandomFloatInRange` -450.0 450.0)) (.location (`self.GetTransform`))) (.rotation (`self.GetTransform`)) (.scale (`self.GetTransform`))) "Undefined" "OverrideRootScale" null null))
  (bind _aspoint_formation (cast `/Game/Blueprints/Points/Prefabs/PointFormation` _returnvalue))
  (`self.SpawnFormation` _aspoint_formation))

(event `self.EndTrigger.OnComponentEndOverlap`
  (params (OverlappedComponent :type "PrimitiveComponent Object Reference") (OtherActor :type "Actor Object Reference") (OtherComp :type "PrimitiveComponent Object Reference") (OtherBodyIndex :type Integer))
  (bind _mypoints (`self.MyPoints`))
  ;[1 1 1] Procedural
  (cast `/Game/Blueprints/RayCharacter` OtherActor)
  (`/Engine/EditorBlueprintResources/StandardMacros.DoOnce` false
    (:`Completed`
      (if (`self.Procedural`)
        (bind _asray_game_mode (cast `/Game/Blueprints/RayGameMode` (`GameplayStatics.GetGameMode`)))
        (`/Game/Blueprints/RayGameMode.AddRandomFloor` _asray_game_mode))
      (`KismetSystemLibrary.Delay` 4.0)
      (for (_array_element _array_index) _mypoints
        (`/Engine/EditorBlueprintResources/StandardMacros.IsValid` _array_element
          (:`Is Valid`
            (`self.K2_DestroyActor` (`|GetArrayItem` (`self.MyPoints`) _array_index)))))
      (`KismetArrayLibrary.Array_Clear` _mypoints)
      (`self.K2_DestroyActor`))))

(fn `SpawnFormation`
  (params (Formatoin :type "/Game/Blueprints/Points/Prefabs/PointFormation Object Reference"))
  (locals (GivenFormation :type "/Game/Blueprints/Points/Prefabs/PointFormation Object Reference"))
  (bind _output_get (set `local.GivenFormation` Formatoin))
  (for _array_element (`self.K2_GetComponentsByClass` _output_get "/Script/Engine.ArrowComponent")
    (bind (_returnvalue_location _returnvalue_rotation _returnvalue_scale) (`KismetMathLibrary.BreakTransform` (`SceneComponent.K2_GetComponentToWorld` _array_element)))
    (bind _returnvalue (`|SpawnActorFromClass` "/Game/Blueprints/Points/Point.Point_C" (`KismetMathLibrary.MakeTransform` _returnvalue_location (struct) _returnvalue_scale) "Undefined" "OverrideRootScale" null null))
    (`KismetArrayLibrary.Array_Add` (`self.MyPoints`) _returnvalue))
  (`self.K2_DestroyActor` (`local.GivenFormation`)))

(fn `UserConstructionScript`
  (`parent.UserConstructionScript`))