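; Floor segment that spawns hazards on BeginPlay: either a black hole or a random meteor formation at a random offset.
; Formations act as disposable templates, with a meteor spawned at each ArrowComponent before the formation is destroyed.
; When RayCharacter first leaves EndTrigger, a procedural floor asks RayGameMode to add a random floor.
; In either mode, the floor destroys its tracked obstacles and itself after a short delay.
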(event `self.ReceiveBeginPlay`
  (bind _returnvalue (`KismetMathLibrary.MakeTransform` (+ (`KismetMathLibrary.MakeVector` (`KismetMathLibrary.RandomFloatInRange` 0.0 450.0) (`KismetMathLibrary.RandomFloatInRange` -450.0 450.0)) (.location (`self.GetTransform`))) (.rotation (`self.GetTransform`)) (.scale (`self.GetTransform`))))
  (if (== (`|GetArrayItem` (`self.Obstacles`) (`KismetMathLibrary.RandomInteger` (`KismetArrayLibrary.Array_Length` (`self.Obstacles`)))) "/Game/Blueprints/Obstacles/BlackHole.BlackHole_C")
    (bind _returnvalue_2 (`|SpawnActorFromClass` "/Game/Blueprints/Obstacles/BlackHole.BlackHole_C" _returnvalue "Undefined" "OverrideRootScale" null null))
    (`KismetArrayLibrary.Array_Add` (`self.Obstacle`) _returnvalue_2)
    (else
      (bind _returnvalue_3 (`|SpawnActorFromClass` (`|GetArrayItem` (`self.Formations`) (`KismetMathLibrary.RandomInteger` (`KismetArrayLibrary.Array_Length` (`self.Formations`)))) _returnvalue "Undefined" "OverrideRootScale" null null))
      (bind _asmeteor_formation (cast `/Game/Blueprints/Obstacles/Prefabs/MeteorFormation` _returnvalue_3))
      (`self.SpawnFormation` _asmeteor_formation))))

(event `self.EndTrigger.OnComponentEndOverlap`
  (params (OverlappedComponent :type "PrimitiveComponent Object Reference") (OtherActor :type "Actor Object Reference") (OtherComp :type "PrimitiveComponent Object Reference") (OtherBodyIndex :type Integer))
  (cast `/Game/Blueprints/RayCharacter` OtherActor)
  (`/Engine/EditorBlueprintResources/StandardMacros.DoOnce` false
    (:`Completed`
      (if (`self.Procedural`)
        (bind _asray_game_mode (cast `/Game/Blueprints/RayGameMode` (`GameplayStatics.GetGameMode`)))
        (`/Game/Blueprints/RayGameMode.AddRandomFloor` _asray_game_mode))
      (`KismetSystemLibrary.Delay` 4.0)
      (for (_array_element _array_index) (`self.Obstacle`)
        (`/Engine/EditorBlueprintResources/StandardMacros.IsValid` _array_element
          (:`Is Valid`
            (`self.K2_DestroyActor` (`|GetArrayItem` (`self.Obstacle`) _array_index)))))
      (`KismetArrayLibrary.Array_Clear` (`self.Obstacle`))
      (`self.K2_DestroyActor`))))

(fn `SpawnFormation`
  (params (Formation :type "/Game/Blueprints/Obstacles/Prefabs/MeteorFormation Object Reference"))
  (locals (GivenFormation :type "/Game/Blueprints/Obstacles/Prefabs/MeteorFormation Object Reference"))
  (bind _output_get (set `local.GivenFormation` Formation))
  (for _array_element (`self.K2_GetComponentsByClass` _output_get "/Script/Engine.ArrowComponent")
    (bind (_returnvalue_location _returnvalue_rotation _returnvalue_scale) (`KismetMathLibrary.BreakTransform` (`SceneComponent.K2_GetComponentToWorld` _array_element)))
    (bind _returnvalue (`|SpawnActorFromClass` "/Game/Blueprints/Obstacles/Meteor.Meteor_C" (`KismetMathLibrary.MakeTransform` _returnvalue_location (struct) _returnvalue_scale) "Undefined" "OverrideRootScale" null null))
    (`KismetArrayLibrary.Array_Add` (`self.Obstacle`) _returnvalue))
  (`self.K2_DestroyActor` (`local.GivenFormation`)))

(fn `UserConstructionScript`
  (`parent.UserConstructionScript`))