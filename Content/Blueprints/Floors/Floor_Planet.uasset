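; Floor_Planet is the level-ending floor piece, where RayCharacter's star points decide victory or game over.
; PlanetTrigger compares points to the character's requirement, then either plays the planet flipbook in slow motion with slowed movement and a victory widget, or pauses on game over.
; Leaving EndTrigger raises speed and RedShift, then after a delay records completion and the next unlock in the Progress game instance and opens NextLevel.
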(event `self.PlanetTrigger.OnComponentBeginOverlap`
  (params (OverlappedComponent :type "PrimitiveComponent Object Reference") (OtherActor :type "Actor Object Reference") (OtherComp :type "PrimitiveComponent Object Reference") (OtherBodyIndex :type Integer) (bFromSweep :type Boolean) (SweepResult :type "HitResult Structure (by ref)"))
  (bind _planetanimation (`self.PlanetAnimation`))
  (bind _asray_character (cast `/Game/Blueprints/RayCharacter` OtherActor))
  (if (>= (`/Game/Blueprints/RayCharacter.Points` _asray_character) (`/Game/Blueprints/RayCharacter.PointsForPlanet` _asray_character))
    (`SceneComponent.SetVisibility` (`self.PlanetSprite`) false false)
    (`SceneComponent.SetVisibility` _planetanimation true false)
    (`PaperFlipbookComponent.PlayFromStart` _planetanimation)
    (`PaperFlipbookComponent.SetLooping` _planetanimation false)
    (`GameplayStatics.SetGlobalTimeDilation` 0.5)
    (set `/Game/Blueprints/RayCharacter.MovementSpeed` 10.0 _asray_character)
    (bind _returnvalue (`|CreateWidget` "/Game/GUI/Victory.Victory_C"))
    (`WidgetLayoutLibrary.RemoveAllWidgets`)
    (`UserWidget.AddToViewport` _returnvalue 0)
    (`GameplayStatics.SpawnSound2D` "/Game/Assets/Sounds/YAY.YAY" 1.0 1.0 0.0 null)
    (else
      (`KismetSystemLibrary.PrintString` "Not Enough Points")
      (bind _returnvalue_2 (`|CreateWidget` "/Game/GUI/GameOver.GameOver_C"))
      (`TextBlock.SetText` (`/Game/GUI/GameOver.additionalText` _returnvalue_2) "You didn't have enough star points")
      (`UserWidget.AddToViewport` _returnvalue_2 0)
      (`GameplayStatics.SetGamePaused` true))))

(event `self.EndTrigger.OnComponentEndOverlap`
  (params (OverlappedComponent :type "PrimitiveComponent Object Reference") (OtherActor :type "Actor Object Reference") (OtherComp :type "PrimitiveComponent Object Reference") (OtherBodyIndex :type Integer))
  (bind _thislevelnumber (`self.ThisLevelNumber`))
  (bind _asray_character (cast `/Game/Blueprints/RayCharacter` OtherActor))
  (set `/Game/Blueprints/RayCharacter.MovementSpeed` 20.0 _asray_character)
  (set `/Game/Blueprints/RayCharacter.RedShift` 100.0 _asray_character)
  (`KismetSystemLibrary.Delay` 2.0)
  (bind _asprogress (cast `/Game/Blueprints/Progress` (`GameplayStatics.GetGameInstance`)))
  (`KismetArrayLibrary.Array_Set` (`/Game/Blueprints/Progress.LevelsCompleted` _asprogress) _thislevelnumber true)
  (`KismetArrayLibrary.Array_Set` (`/Game/Blueprints/Progress.LevelsUnlocked` _asprogress) (+ _thislevelnumber 1) true)
  (`GameplayStatics.OpenLevel` (`KismetStringLibrary.Conv_StringToName` (`self.NextLevel`))))

(event `self.PlanetAnimation.OnFinishedPlaying`
  (`GameplayStatics.SetGlobalTimeDilation` 1.0))

(fn `UserConstructionScript`
  (`parent.UserConstructionScript`))