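; Game mode that builds the level track from chained floor actors, seeding plain then random floors at BeginPlay when Procedural is set.
; Each spawned floor's attach transform becomes the next spawn point.
; AddPlanet places a planet floor plus plain floor and sets End, blocking further random or planet additions.
; MakeLevel builds from a floor pattern array, but its Level1 call is unconnected.
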(event `self.ReceiveBeginPlay`
  ;[1 1 1] Add Floor
  (`KismetSystemLibrary.ControlScreensaver` false)
  (if (`self.Procedural`)
    (for _index (range 6)
      (if (<= _index 2)
        (`self.AddFloor` "/Game/Blueprints/Floors/Floor.Floor_C")
        (else
          (`self.AddRandomFloor`))))))

(fn `AddFloor`
  (params (Floor :type "/Game/Blueprints/Floors/Floor Class Reference"))
  (returns (MadeFloor :type "/Game/Blueprints/Floors/Floor Object Reference"))
  (bind _returnvalue (`|SpawnActorFromClass` Floor (`self.NextSpawnPoint`) "Undefined" "OverrideRootScale" null null))
  (if (`self.Procedural`)
    (set `/Game/Blueprints/Floors/Floor.Procedural` true _returnvalue))
  (bind _attachtransform (`/Game/Blueprints/Floors/Floor.GetAttachTransform` _returnvalue))
  (set `self.NextSpawnPoint` _attachtransform)
  (return _returnvalue))

(fn `AddPlanet`
  (returns (Planet :type "/Game/Blueprints/Floors/Floor_Planet Object Reference"))
  (if (not (`self.End`))
    (bind _returnvalue (`|SpawnActorFromClass` "/Game/Blueprints/Floors/Floor_Planet.Floor_Planet_C" (`self.NextSpawnPoint`) "Undefined" "OverrideRootScale" null null))
    (if (`self.Procedural`)
      (set `/Game/Blueprints/Floors/Floor.Procedural` true _returnvalue))
    (bind _attachtransform (`/Game/Blueprints/Floors/Floor.GetAttachTransform` _returnvalue))
    (set `self.NextSpawnPoint` _attachtransform)
    (for _ (range 4)
      (`self.AddFloor` "/Game/Blueprints/Floors/Floor.Floor_C")
      (set `self.End` true)
      (return _returnvalue))))

(fn `AddRandomFloor`
  (locals (Floors :type "Array of /Game/Blueprints/Floors/Floor Class Reference"))
  (if (not (`self.End`))
    (bind _returnvalue (`|SpawnActorFromClass` (`|GetArrayItem` (`local.Floors`) (`KismetMathLibrary.RandomInteger` (`KismetArrayLibrary.Array_Length` (`local.Floors`)))) (`self.NextSpawnPoint`) "Undefined" "OverrideRootScale" null null))
    (if (`self.Procedural`)
      (set `/Game/Blueprints/Floors/Floor.Procedural` true _returnvalue))
    (bind _attachtransform (`/Game/Blueprints/Floors/Floor.GetAttachTransform` _returnvalue))
    (set `self.NextSpawnPoint` _attachtransform)))

(fn `MakeLevel`
  (params (Pattern :type "Array of /Game/Blueprints/Floors/Floor Class Reference"))
  (returns (Floors :type "Array of /Game/Blueprints/Floors/Floor Object Reference"))
  (locals (FloorsMade :type "Array of /Game/Blueprints/Floors/Floor Object Reference"))
  (for _array_element Pattern
    (bind _madefloor (`self.AddFloor` _array_element))
    (`KismetArrayLibrary.Array_Add` (`local.FloorsMade`) _madefloor))
  (return (`local.FloorsMade`)))

(fn `UserConstructionScript`)