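; Meteor obstacle that either explodes or ends the game when the RayCharacter overlaps its Sphere1 collision, guarded by a Hit flag.
; In PowerMode it swaps the asteroid sprite for a one-shot explosion animation with controller rumble, then destroys itself when playback finishes.
; Otherwise it shows the GameOver widget and pauses the game.
; Disconnected leftover logic covers point loss, PowerMode reset and level reload.
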(event `self.Sphere.OnComponentHit`
  (params (HitComponent :type "PrimitiveComponent Object Reference") (OtherActor :type "Actor Object Reference") (OtherComp :type "PrimitiveComponent Object Reference") (NormalImpulse :type "Vector Structure") (Hit :type "HitResult Structure (by ref)")))

(event `self.Sphere1.OnComponentBeginOverlap`
  (params (OverlappedComponent :type "PrimitiveComponent Object Reference") (OtherActor :type "Actor Object Reference") (OtherComp :type "PrimitiveComponent Object Reference") (OtherBodyIndex :type Integer) (bFromSweep :type Boolean) (SweepResult :type "HitResult Structure (by ref)"))
  (bind _asteroid_animation (`self.asteroid_animation`))
  (if (not (`self.Hit`))
    (bind _asray_character (cast `/Game/Blueprints/RayCharacter` OtherActor))
    (set `self.Hit` true)
    (if (`/Game/Blueprints/RayCharacter.PowerMode` _asray_character)
      (`KismetSystemLibrary.PrintString` "Boom!" false)
      (`SceneComponent.SetVisibility` (`self.asteroid_Sprite`) false false)
      (`SceneComponent.SetVisibility` _asteroid_animation true false)
      (`PaperFlipbookComponent.PlayFromStart` _asteroid_animation)
      (`PaperFlipbookComponent.SetLooping` _asteroid_animation false)
      (`PlayerController.PlayDynamicForceFeedback` (`GameplayStatics.GetPlayerController` 0) 0.3 0.5 true true true true)
      (else
        (bind _returnvalue (`|CreateWidget` "/Game/GUI/GameOver.GameOver_C"))
        (`UserWidget.AddToViewport` _returnvalue 0)
        (`GameplayStatics.SetGamePaused` true)))))

(event `self.ReceiveActorBeginOverlap`
  (params (OtherActor :type "Actor Object Reference")))

(event `self.asteroid_animation.OnFinishedPlaying`
  (`self.K2_DestroyActor`))

(fn `UserConstructionScript`)